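; BP_Void1 handles basic session setup and a countdown that depends on the Pyromaniac AI.
; BeginPlay caps the frame rate, hides the mouse cursor, caches the first BP_Pyromaniac and starts a looping one-second timer.
; While that actor's AI controller has DoBehaviorTree set, UpdateTime derives Minutes and Seconds from the remaining time and decrements it until zero.
; Pressing Escape quits the game.
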(event EventTick
  (params (DeltaSeconds :type Float%20%28single-precision%29)))

(event EventBeginPlay
  (Development|ExecuteConsoleCommand "t.MaxFps 60" 0)
  (Variables|/Script/Engine.PlayerController|SetbShowMouseCursor (Game|GetPlayerController 0) false)
  (Utilities|Time|SetTimerbyFunctionName 0 "UpdateTime" 1.0 true)
  (bind _outactors (Actor|GetAllActorsOfClass "/Game/TFD/Imade/Blueprints/BP_Pyromaniac.BP_Pyromaniac_C"))
  (Variables|Default|SetPyromaniacRef (Utilities|Array|Get(acopy) _outactors)))

(event Input|KeyboardEvents|Escape
  (params (Key :type Key%20Structure :default "None"))
  (:Pressed
    (Game|QuitGame 0 "Quit" false)))

(fn ConstructionScript)

(fn UpdateTime
  (bind _asaic_pyromaniac (Utilities|Casting|CastToAIC_Pyromaniac (AI|GetAIController (Variables|Default|GetPyromaniacRef))))
  (if (Variables|/Game/TFD/Imade/Blueprints/Controllers/AIC_Pyromaniac.AIC_Pyromaniac_C|GetDoBehaviorTree _asaic_pyromaniac)
    (if (not (<= (Variables|Default|GetTimeRemaing) 0.0))
      (Variables|Default|SetMinutes (Math|Float|Truncate (/ (Variables|Default|GetTimeRemaing) 6e+01)))
      (Variables|Default|SetSeconds (Math|Float|Truncate (Math|Float|%(Float) (Variables|Default|GetTimeRemaing) 6e+01)))
      (Variables|Default|SetTimeRemaing (- (Variables|Default|GetTimeRemaing) 1.0))
      (return))))