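; BP_HandCanonBullet is a hand cannon bullet that deals point damage to BP_Pyromaniac1 on hit, ignoring other actors.
; The hit bone selects a critical threshold: fixed for head shell, clavicle and core weakness bones, otherwise from GetCriticalHitChance.
; A random roll at or above that threshold multiplies damage by the critical multiplier, so a higher threshold means fewer crits.
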(event Collision|EventHit
  (params (MyComp :type Primitive%20Component%20Object%20Reference) (Other :type Actor%20Object%20Reference) (OtherComp :type Primitive%20Component%20Object%20Reference) (bSelfMoved :type Boolean) (HitLocation :type Vector :default "0, 0, 0") (HitNormal :type Vector :default "0, 0, 0") (NormalImpulse :type Vector :default "0, 0, 0") (Hit :type Hit%20Result%20Structure%20%28by%20ref%29))
  (bind _asbp_pyromaniac (Utilities|Casting|CastToBP_Pyromaniac1 Other))
  (switch name (.BoneName (Collision|BreakHitResult Hit))
    (:Default
      (if (<= (Variables|Default|GetGetCriticalHitChance%20) (Math|Random|RandomFloatinRange 0.0 1.0))
        (Game|Damage|ApplyPointDamage _asbp_pyromaniac (* (Variables|Default|GetGetDamage) (Variables|Default|GetGetCirticalDamage)) (Math|Vector|GetForwardVector (Transformation|GetActorRotation)) Hit 0 self)
        (else
          (Game|Damage|ApplyPointDamage _asbp_pyromaniac (Variables|Default|GetGetDamage) (Math|Vector|GetForwardVector (Transformation|GetActorRotation)) Hit 0 self))))
    (:Dm_RealCore_Weakness
      (if (<= 0.8 (Math|Random|RandomFloatinRange 0.0 1.0)) :!label _label
        (Game|Damage|ApplyPointDamage _asbp_pyromaniac (* (Variables|Default|GetGetDamage) (Variables|Default|GetGetCirticalDamage)) (Math|Vector|GetForwardVector (Transformation|GetActorRotation)) Hit 0 self)
        (else
          (Game|Damage|ApplyPointDamage _asbp_pyromaniac (Variables|Default|GetGetDamage) (Math|Vector|GetForwardVector (Transformation|GetActorRotation)) Hit 0 self))))
    (:Dm_HeadShell_L_Weakness
      (goto _label))
    (:Dm_HeadShell_R_Weakness
      (goto _label))
    (:Dm_Clav_L_Weakness
      (goto _label))
    (:Dm_Clav_R_Weakness
      (goto _label))))

(fn ConstructionScript
  (|CallParentFunction))