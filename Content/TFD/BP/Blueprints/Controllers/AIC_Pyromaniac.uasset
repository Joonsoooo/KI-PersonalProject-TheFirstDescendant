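; AI controller for the Pyromaniac that runs its behavior tree and keeps focus on the blackboard's ClosestPlayer.
; RunBehavior possesses the pawn, starts BT_Pyromaniac and enables the Tick logic, but nothing in this file's live graph calls it.
; Tick refreshes focus, then passes a DoOnce that resets while SkillActive is true.
; Once it is false, a random normal-mode skill chance is written to the blackboard and the gate stays closed.
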(event EventTick
  (params (DeltaSeconds :type Float%20%28single-precision%29))
  (if (Variables|Default|GetDoBehaviorTree)
    (bind _as액터 (Utilities|Casting|CastToActor (AI|Components|Blackboard|GetValueasObject (AI|GetBlackboard 0) (Utilities|Name|MakeLiteralName "ClosestPlayer"))))
    (AI|SetFocus _as액터)
    (CallFunction|RandomSkillChanceNormalMode)))

(fn ConstructionScript)

(fn RandomSkillChanceNormalMode
  (Utilities|FlowControl|DoOnce false :!label _label
    (:Completed
      (if (ScalableFloat|GetValueasBool (AI|GetBlackboard 0) (Utilities|Name|MakeLiteralName "SkillActive"))
        (goto _label Reset)
        (else
          (AI|Components|Blackboard|SetValueasFloat (AI|GetBlackboard 0) (Utilities|Name|MakeLiteralName "RandomSkillChance_NormalMode") (Math|Random|RandomFloatinRange 0.0 1.2))
          (return))))))

(fn RunBehavior
  (Pawn|Possess (Pawn|GetControlledPawn))
  (AI|RunBehaviorTree "/Game/TFD/Imade/Blueprints/BehaviorTree/BT_Pyromaniac.BT_Pyromaniac")
  (Variables|Default|SetDoBehaviorTree true)
  (bind _as액터 (Utilities|Casting|CastToActor (AI|Components|Blackboard|GetValueasObject (AI|GetBlackboard 0) (Utilities|Name|MakeLiteralName "ClosestPlayer"))))
  (AI|SetFocus _as액터)
  (return))