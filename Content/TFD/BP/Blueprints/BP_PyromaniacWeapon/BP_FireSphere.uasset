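; BP_FireSphere is a Pyromaniac weapon fire sphere that damages what it overlaps and shoots smaller flames at a target player.
; Overlap spawns a hit effect, applies damage and destroys it; a hit or lifetime timeout also destroys it.
; Tick feeds a Delay, throttling FireSmallFlame to roughly half-second intervals.
; When TargetPlayer is valid and nearby, it launches BP_FireSphereSmallFlame toward the spine socket, homing on the root component.
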(event OnComponentBeginOverlap(Sphere)
  (params (OverlappedComponent :type Primitive%20Component%20Object%20Reference) (OtherActor :type Actor%20Object%20Reference) (OtherComp :type Primitive%20Component%20Object%20Reference) (OtherBodyIndex :type Integer) (bFromSweep :type Boolean) (SweepResult :type Hit%20Result%20Structure%20%28by%20ref%29))
  (Niagara|SpawnSystematLocation "/Game/TFD/Imade/VFX/NS_FlameHit.NS_FlameHit" (.Location (Collision|BreakHitResult SweepResult)))
  (Game|Damage|ApplyDamage OtherActor 8e+01 0 self)
  (Actor|DestroyActor))

(event OnComponentHit(Sphere)
  (params (HitComponent :type Primitive%20Component%20Object%20Reference) (OtherActor :type Actor%20Object%20Reference) (OtherComp :type Primitive%20Component%20Object%20Reference) (NormalImpulse :type Vector :default "0, 0, 0") (Hit :type Hit%20Result%20Structure%20%28by%20ref%29))
  (Actor|DestroyActor))

(event Custom|SmallFlameDelay
  (Utilities|FlowControl|Delay 0.5)
  (CallFunction|FireSmallFlame))

(event EventTick
  (params (DeltaSeconds :type Float%20%28single-precision%29))
  (CallFunction|SmallFlameDelay))

(event EventBeginPlay
  (Utilities|FlowControl|Delay 4.0)
  (Actor|DestroyActor))

(fn ConstructionScript)

(fn FireSmallFlame
  (bind _returnvalue (Transformation|GetActorLocation))
  (bind _targetplayer (Variables|Default|GetTargetPlayer)
    (:then
      (if (<= (Math|Vector|Distance(Vector) _returnvalue (Transformation|GetActorLocation _targetplayer)) 7e+02)
        (bind _returnvalue_2 (Game|SpawnActorfromClass "/Game/TFD/Imade/Blueprints/BP_PyromaniacWeapon/BP_FireSphereSmallFlame.BP_FireSphereSmallFlame_C" (Math|Transform|MakeTransform _returnvalue (Math|Rotator|FindLookatRotation _returnvalue (Transformation|GetSocketLocation (Variables|/Script/Engine.Actor|GetRootComponent _targetplayer) "Bip001-Spine3"))) "Undefined" 0 0))
        (Variables|/Script/Engine.MovementComponent|SetVelocity (Variables|/Game/TFD/Imade/Blueprints/BP_PyromaniacWeapon/BP_FireSphereSmallFlame.BP_FireSphereSmallFlame_C|GetProjectileMovement _returnvalue_2) (* (Math|Vector|GetForwardVector (.Rotation (Math|Transform|BreakTransform (Math|Transform|MakeTransform _returnvalue (Math|Rotator|FindLookatRotation _returnvalue (Transformation|GetSocketLocation (Variables|/Script/Engine.Actor|GetRootComponent _targetplayer) "Bip001-Spine3")))))) 5e+03))
        (Variables|/Script/Engine.ProjectileMovementComponent|SetHomingTargetComponent (Variables|/Game/TFD/Imade/Blueprints/BP_PyromaniacWeapon/BP_FireSphereSmallFlame.BP_FireSphereSmallFlame_C|GetProjectileMovement _returnvalue_2) (Variables|/Script/Engine.Actor|GetRootComponent (Variables|Default|GetTargetPlayer)))
        (return)))
    (:else)))