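; BP_FlameNet is a short-lived Pyromaniac weapon actor that destroys itself one second after BeginPlay.
; SetLocationAndLength traces down from StartLocation on Visibility, falling back to a fixed depth on a miss, to find GroundLocation.
; It places the static mesh at StartLocation and scales its Z by the drop distance, assuming a 100-unit mesh.
; The event graph's only call to this function is unconnected.
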(event EventBeginPlay
  (Utilities|FlowControl|Delay 1.0)
  (Actor|DestroyActor))

(event EventTick
  (params (DeltaSeconds :type Float%20%28single-precision%29)))

(fn ConstructionScript)

(fn SetLocationandLength
  (bind _startlocation (Variables|Default|GetStartLocation))
  (bind _startlocation_2 (Variables|Default|GetStartLocation))
  (bind _staticmesh (Variables|Default|GetStaticMesh))
  (bind _returnvalue (- _startlocation "0.000000,0.000000,2000.000000"))
  (bind _outhit (Collision|LineTraceByChannel _startlocation _returnvalue "TraceTypeQuery1" false 0 "None"))
  (if (.bBlockingHit (Collision|BreakHitResult _outhit))
    (bind _output_get (Variables|Default|SetGroundLocation (.Location (Collision|BreakHitResult _outhit))))
    (Variables|Default|SetDistanceStartLocationToGroundLocation (Math|Vector|VectorLength (- _output_get _startlocation_2)))
    (else
      (bind _output_get_2 (Variables|Default|SetGroundLocation _returnvalue))
      (Variables|Default|SetDistanceStartLocationToGroundLocation (Math|Vector|VectorLength (- _output_get_2 _startlocation_2)))))
  (Transformation|SetWorldLocation _staticmesh (Variables|Default|GetStartLocation) false false)
  (Transformation|SetWorldScale3D _staticmesh (Math|Vector|MakeVector 1.0 1.0 (/ (Variables|Default|GetDistanceStartLocationToGroundLocation) 1e+02)))
  (return))