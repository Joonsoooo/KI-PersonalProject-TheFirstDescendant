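; Short-lived flamethrower attack actor for the Pyromaniac weapon that spans from its spawn location toward a target player.
; After a brief delay, it sizes and centers a capsule hitbox between the two points and scales the Niagara flame by their distance.
; Actors that begin overlapping the capsule take fixed damage and show a hit effect at the sweep impact point.
; The actor destroys itself shortly afterward.
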(event OnComponentBeginOverlap(Capsule)
  (params (OverlappedComponent :type Primitive%20Component%20Object%20Reference) (OtherActor :type Actor%20Object%20Reference) (OtherComp :type Primitive%20Component%20Object%20Reference) (OtherBodyIndex :type Integer) (bFromSweep :type Boolean) (SweepResult :type Hit%20Result%20Structure%20%28by%20ref%29))
  (Niagara|SpawnSystematLocation "/Game/TFD/Imade/VFX/NS_FlameHit.NS_FlameHit" (.ImpactPoint (Collision|BreakHitResult SweepResult)) "0, 0, 0" "1.000000,1.000000,1.000000" true true "None" false)
  (Game|Damage|ApplyDamage OtherActor 1e+01 0 0))

(event EventTick
  (params (DeltaSeconds :type Float%20%28single-precision%29)))

(event EventBeginPlay
  (bind _targetplayer (Variables|Default|GetTargetPlayer))
  (bind _capsule (Variables|Default|GetCapsule))
  (bind _niagara (Variables|Default|GetNiagara))
  (bind _spawnlocation (Variables|Default|GetSpawnLocation))
  (bind _returnvalue (Transformation|GetActorLocation _targetplayer))
  (bind _returnvalue_2 (- _returnvalue _spawnlocation))
  (bind _returnvalue_3 (Math|Vector|VectorLength _returnvalue_2))
  (Utilities|FlowControl|Delay 0.2)
  (Components|Capsule|SetCapsuleHalfHeight _capsule (/ _returnvalue_3 2.1) true)
  (Components|Capsule|SetCapsuleRadius _capsule 1.5e+02 true)
  (Transformation|SetActorLocation (+ (/ _returnvalue_2 2.1) (Variables|Default|GetSpawnLocation)) false false)
  (Transformation|SetWorldLocation _niagara _spawnlocation false false)
  (Niagara|SetNiagaraVariable(Float) _niagara "SetScale" _returnvalue_3)
  (Niagara|SetNiagaraVariable(Float) _niagara "SetLength" (* _returnvalue_3 3.0))
  (Utilities|FlowControl|Delay 0.5)
  (Actor|DestroyActor))

(fn ConstructionScript)