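; Flame ring actor in the Pyromaniac weapon set that expands horizontally and damages what it touches.
; On BeginPlay the SetScale timeline adds to the actor's X and Y scale every update, with the Niagara effect set to a quarter of that scale.
; Static mesh overlaps spawn a flame hit effect at the sweep impact point and apply fixed damage to the other actor.
; The ring destroys itself after a fixed delay.
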(event OnComponentBeginOverlap(StaticMesh)
  (params (OverlappedComponent :type Primitive%20Component%20Object%20Reference) (OtherActor :type Actor%20Object%20Reference) (OtherComp :type Primitive%20Component%20Object%20Reference) (OtherBodyIndex :type Integer) (bFromSweep :type Boolean) (SweepResult :type Hit%20Result%20Structure%20%28by%20ref%29))
  (Niagara|SpawnSystematLocation "/Game/TFD/Imade/VFX/NS_FlameHit.NS_FlameHit" (.ImpactPoint (Collision|BreakHitResult SweepResult)))
  (Game|Damage|ApplyDamage OtherActor 5e+01 0 0))

(event EventBeginPlay
  (Utilities|FlowControl|Sequence
    (:then_0
      (Utilities|FlowControl|Delay 1e+01)
      (Actor|DestroyActor))
    (:then_1
      (bind _새_트랙_0 (Timeline|SetScale PlayFromStart)
        (:Update
          (Transformation|SetActorScale3D (+ (Transformation|GetActorScale3D) (Math|Vector|MakeVector _새_트랙_0 _새_트랙_0 0.0) ""))
          (Transformation|SetWorldScale3D (Variables|Default|GetNiagara) (/ (+ (Transformation|GetActorScale3D) (Math|Vector|MakeVector _새_트랙_0 _새_트랙_0 0.0) "") 4.0)))))))

(fn ConstructionScript)