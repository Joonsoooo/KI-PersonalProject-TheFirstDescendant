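; Pyromaniac boss enemy character that plays a spawn montage and fights with flame and minion-summon skills through an AIC_Pyromaniac behavior tree.
; Each tick it copies its normal/berserk mode to the Blackboard, clears skill cooldown flags after delays, and pitches waist and neck toward the player.
; Point damage routes by bone name to weakness or body handlers, which roll criticals and subtract weapon damage from Shield, then Hp.
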(event EventBeginPlay
  (Animation|Montage|PlayMontage (Variables|Character|GetMesh) "/Game/TFD/Imade/Blueprints/Animation/Montages/Pyromaniac1/AM_Spawn1.AM_Spawn1"))

(event EventTick
  (params (DeltaSeconds :type Float%20%28single-precision%29))
  (CallFunction|ManageSkillsCooltime)
  (CallFunction|SetMode)
  (CallFunction|SetPitch))

(event Game|Damage|EventPointDamage
  (params (Damage :type Float%20%28single-precision%29) (DamageType :type Damage%20Type%20Object%20Reference) (HitLocation :type Vector :default "0, 0, 0") (HitNormal :type Vector :default "0, 0, 0") (HitComponent :type Primitive%20Component%20Object%20Reference) (BoneName :type Name :default "None") (ShotFromDirection :type Vector :default "0, 0, 0") (InstigatedBy :type Controller%20Object%20Reference) (DamageCauser :type Actor%20Object%20Reference) (HitInfo :type Hit%20Result%20Structure%20%28by%20ref%29))
  (switch name BoneName
    (:Default
      (CallFunction|LineTraceTakeDamage DamageCauser))
    (:Dm_Knee_L_Weakness
      (CallFunction|LineTraceWeaknessTakeDamage DamageCauser :!label _label))
    (:Dm_Knee_R_Weakness
      (goto _label))
    (:Dm_Clav_L_Weakness
      (goto _label))
    (:Dm_Clav_R_Weakness
      (goto _label))
    (:Dm_HeadShell_L_Weakness
      (goto _label))
    (:Dm_HeadShell_R_Weakness
      (goto _label))
    (:Dm_RealCore_Weakness
      (goto _label))))

(event Custom|Manage%20Skills%20Cooltime
  (bind _returnvalue (AI|GetBlackboard 0))
  (bind _returnvalue_2 (Utilities|Name|MakeLiteralName "CoolTime_BerserkSummonMinions"))
  (bind _returnvalue_3 (AI|GetBlackboard 0))
  (bind _returnvalue_4 (Utilities|Name|MakeLiteralName "CoolTime_FlameThrow"))
  (bind _returnvalue_5 (AI|GetBlackboard 0))
  (bind _returnvalue_6 (Utilities|Name|MakeLiteralName "CoolTime_GroundBurster"))
  (bind _returnvalue_7 (AI|GetBlackboard 0))
  (bind _returnvalue_8 (Utilities|Name|MakeLiteralName "CoolTime_NormalSummonMinions"))
  (bind _returnvalue_9 (AI|GetBlackboard 0))
  (bind _returnvalue_10 (Utilities|Name|MakeLiteralName "CoolTime_SummonFlyMinions"))
  (bind _returnvalue_11 (AI|GetBlackboard 0))
  (bind _returnvalue_12 (Utilities|Name|MakeLiteralName "CoolTime_FlameShot"))
  (bind _returnvalue_13 (AI|GetBlackboard 0))
  (bind _returnvalue_14 (Utilities|Name|MakeLiteralName "CoolTime_FlameNet"))
  (bind _returnvalue_15 (AI|GetBlackboard 0))
  (bind _returnvalue_16 (Utilities|Name|MakeLiteralName "CoolTime_FTO"))
  (bind _returnvalue_17 (AI|GetBlackboard 0))
  (bind _returnvalue_18 (Utilities|Name|MakeLiteralName "CoolTime_FTO"))
  (bind _returnvalue_19 (AI|GetBlackboard 0))
  (bind _returnvalue_20 (Utilities|Name|MakeLiteralName "CoolTime_BusterCall"))
  (bind _run_bt (CallFunction|DoBehaviorTree))
  (if _run_bt
    (if (== (Variables|Default|GetCurrentMode) 0)
      (if (ScalableFloat|GetValueasBool _returnvalue_11 _returnvalue_12)
        (Utilities|FlowControl|Delay 5.0)
        (AI|Components|Blackboard|SetValueasBool _returnvalue_11 _returnvalue_12 false)
        (elif (ScalableFloat|GetValueasBool _returnvalue_3 _returnvalue_4)
          (Utilities|FlowControl|Delay 5.0)
          (AI|Components|Blackboard|SetValueasBool _returnvalue_3 _returnvalue_4 false)
          (elif true
            (Utilities|FlowControl|Delay 5.0)
            (AI|Components|Blackboard|SetValueasBool (AI|GetBlackboard 0) (Utilities|Name|MakeLiteralName "CoolTime_FireSphere") false)
            (elif (ScalableFloat|GetValueasBool _returnvalue_5 _returnvalue_6)
              (Utilities|FlowControl|Delay 5.0)
              (AI|Components|Blackboard|SetValueasBool _returnvalue_5 _returnvalue_6 false)
              (elif (ScalableFloat|GetValueasBool _returnvalue_7 _returnvalue_8)
                (Utilities|FlowControl|Delay 2e+01)
                (AI|Components|Blackboard|SetValueasBool _returnvalue_7 _returnvalue_8 false)
                (elif (not true)
                  (if (ScalableFloat|GetValueasBool _returnvalue_9 _returnvalue_10)
                    (Utilities|FlowControl|Delay 6e+01)
                    (AI|Components|Blackboard|SetValueasBool _returnvalue_9 _returnvalue_10 false))))))))
      (elif (ScalableFloat|GetValueasBool _returnvalue_13 _returnvalue_14)
        (Utilities|FlowControl|Delay 5.0)
        (AI|Components|Blackboard|SetValueasBool _returnvalue_13 _returnvalue_14 false)
        (elif (ScalableFloat|GetValueasBool _returnvalue_15 _returnvalue_16)
          (Utilities|FlowControl|Delay 5.0)
          (AI|Components|Blackboard|SetValueasBool _returnvalue_15 _returnvalue_16 false)
          (elif (ScalableFloat|GetValueasBool _returnvalue_17 _returnvalue_18)
            (Utilities|FlowControl|Delay 5.0)
            (AI|Components|Blackboard|SetValueasBool _returnvalue_17 _returnvalue_18 false)
            (elif (ScalableFloat|GetValueasBool _returnvalue_19 _returnvalue_20)
              (Utilities|FlowControl|Delay 5.0)
              (AI|Components|Blackboard|SetValueasBool _returnvalue_19 _returnvalue_20 false)
              (elif (ScalableFloat|GetValueasBool _returnvalue _returnvalue_2)
                (Utilities|FlowControl|Delay 2e+01)
                (AI|Components|Blackboard|SetValueasBool _returnvalue _returnvalue_2 false)))))))))

(fn ConstructionScript)

(fn SetMode
  (bind _run_bt (CallFunction|DoBehaviorTree))
  (if _run_bt
    (AI|Components|Blackboard|SetValueasEnum (AI|GetBlackboard 0) (Utilities|Name|MakeLiteralName "CurrentMode") (Variables|Default|GetCurrentMode))
    (return)))

(fn DoBehaviorTree
  (bind _asaic_pyromaniac (Utilities|Casting|CastToAIC_Pyromaniac (AI|GetAIController self)))
  (if (Variables|/Game/TFD/Imade/Blueprints/Controllers/AIC_Pyromaniac.AIC_Pyromaniac_C|GetDoBehaviorTree _asaic_pyromaniac)
    (return true)))

(fn SetPitch
  (Variables|Default|SetWaistPitch (.Pitch (Math|Rotator|BreakRotator (Math|Rotator|FindLookatRotation (Transformation|GetSocketLocation (Variables|Character|GetMesh) "EyeSocket") (Transformation|GetWorldLocation (Variables|/Script/Engine.Actor|GetRootComponent (Game|GetPlayerCharacter 0)))))))
  (Variables|Default|SetNeckPitch (.Pitch (Math|Rotator|BreakRotator (Math|Rotator|FindLookatRotation (Transformation|GetSocketLocation (Variables|Character|GetMesh) "NeckSocket") (Transformation|GetWorldLocation (Variables|/Script/Engine.Actor|GetRootComponent (Game|GetPlayerCharacter 0)))))))
  (return))

(fn TakeDamage
  (params (Attacker :type Actor%20Object%20Reference))
  (if (!= Attacker self)
    (bind _asbp_bullet_base (Utilities|Casting|CastToBP_BulletBase Attacker))
    (Variables|Default|SetWeaknessHit true)
    (Development|PrintString "Critical")
    (switch Utilities|FlowControl|Switch|SwitchonBULLET_TYPE (Variables|/Game/TFD/Imade/Blueprints/BaseBlueprints/BP_BulletBase.BP_BulletBase_C|GetBulletType _asbp_bullet_base)
      (:NewEnumerator0
        _)
      (:NewEnumerator1
        _)
      (:NewEnumerator2
        _))
    (if (<= 0.7 (Math|Random|RandomFloatinRange 0.0 1.0))
      (Variables|/Game/TFD/Imade/Blueprints/BaseBlueprints/BP_BulletBase.BP_BulletBase_C|SetGetCriticalHit _asbp_bullet_base true)
      (if (>= (Variables|Default|GetShield) 0.0)
        (Variables|Default|SetShield (- (Variables|Default|GetShield) (* (Variables|/Game/TFD/Imade/Blueprints/BaseBlueprints/BP_BulletBase.BP_BulletBase_C|GetGetDamage _asbp_bullet_base) (Variables|/Game/TFD/Imade/Blueprints/BaseBlueprints/BP_BulletBase.BP_BulletBase_C|GetGetCirticalDamage _asbp_bullet_base))))
        (Variables|Default|SetWeaknessHit false :!label _label)
        (Actor|DestroyActor _asbp_bullet_base)
        (return)
        (elif (>= (Variables|Default|GetHp) 0.0)
          (Variables|Default|SetHp (- (Variables|Default|GetHp) (* (Variables|/Game/TFD/Imade/Blueprints/BaseBlueprints/BP_BulletBase.BP_BulletBase_C|GetGetDamage _asbp_bullet_base) (Variables|/Game/TFD/Imade/Blueprints/BaseBlueprints/BP_BulletBase.BP_BulletBase_C|GetGetCirticalDamage _asbp_bullet_base))))
          (goto _label)))
      (else
        (Variables|/Game/TFD/Imade/Blueprints/BaseBlueprints/BP_BulletBase.BP_BulletBase_C|SetGetCriticalHit _asbp_bullet_base false)
        (if (>= (Variables|Default|GetShield) 0.0)
          (Variables|Default|SetShield (- (Variables|Default|GetShield) (Variables|/Game/TFD/Imade/Blueprints/BaseBlueprints/BP_BulletBase.BP_BulletBase_C|GetGetDamage _asbp_bullet_base)))
          (goto _label)
          (elif (>= (Variables|Default|GetHp) 0.0)
            (Variables|Default|SetHp (- (Variables|Default|GetHp) (Variables|/Game/TFD/Imade/Blueprints/BaseBlueprints/BP_BulletBase.BP_BulletBase_C|GetGetDamage _asbp_bullet_base)))
            (goto _label)))))))

(fn LineTraceWeaknessTakeDamage
  (params (AttackCauser :type Actor%20Object%20Reference))
  (bind _asbp_weapon_base (Utilities|Casting|CastToBP_WeaponBase AttackCauser))
  (Variables|Default|SetWeaknessHit true)
  (Development|PrintString "Critical")
  (if (<= 0.7 (Math|Random|RandomFloatinRange 0.0 1.0))
    (Variables|/Game/TFD/Imade/Blueprints/BaseBlueprints/BP_WeaponBase.BP_WeaponBase_C|SetCirticalHit _asbp_weapon_base true)
    (if (>= (Variables|Default|GetShield) 0.0)
      (Variables|Default|SetShield (- (Variables|Default|GetShield) (* (Variables|/Game/TFD/Imade/Blueprints/BaseBlueprints/BP_WeaponBase.BP_WeaponBase_C|GetDamage _asbp_weapon_base) (Variables|/Game/TFD/Imade/Blueprints/BaseBlueprints/BP_WeaponBase.BP_WeaponBase_C|GetCirticalDamage _asbp_weapon_base))))
      (Variables|Default|SetWeaknessHit false :!label _label)
      (return)
      (elif (>= (Variables|Default|GetHp) 0.0)
        (Variables|Default|SetHp (- (Variables|Default|GetHp) (* (Variables|/Game/TFD/Imade/Blueprints/BaseBlueprints/BP_WeaponBase.BP_WeaponBase_C|GetDamage _asbp_weapon_base) (Variables|/Game/TFD/Imade/Blueprints/BaseBlueprints/BP_WeaponBase.BP_WeaponBase_C|GetCirticalDamage _asbp_weapon_base))))
        (goto _label)))
    (else
      (Variables|/Game/TFD/Imade/Blueprints/BaseBlueprints/BP_WeaponBase.BP_WeaponBase_C|SetCirticalHit _asbp_weapon_base false)
      (if (>= (Variables|Default|GetShield) 0.0)
        (Variables|Default|SetShield (- (Variables|Default|GetShield) (Variables|/Game/TFD/Imade/Blueprints/BaseBlueprints/BP_WeaponBase.BP_WeaponBase_C|GetDamage _asbp_weapon_base)))
        (goto _label)
        (elif (>= (Variables|Default|GetHp) 0.0)
          (Variables|Default|SetHp (- (Variables|Default|GetHp) (Variables|/Game/TFD/Imade/Blueprints/BaseBlueprints/BP_WeaponBase.BP_WeaponBase_C|GetDamage _asbp_weapon_base)))
          (goto _label))))))

(fn LineTraceTakeDamage
  (params (AttackCauser :type Actor%20Object%20Reference))
  (if (not (Variables|Default|GetWeaknessHit))
    (bind _asbp_weapon_base (Utilities|Casting|CastToBP_WeaponBase AttackCauser))
    (Development|PrintString "Defalut")
    (if (<= 0.1 (Math|Random|RandomFloatinRange 0.0 1.0))
      (Variables|/Game/TFD/Imade/Blueprints/BaseBlueprints/BP_WeaponBase.BP_WeaponBase_C|SetCirticalHit _asbp_weapon_base true)
      (if (>= (Variables|Default|GetShield) 0.0)
        (Variables|Default|SetShield (- (Variables|Default|GetShield) (* (Variables|/Game/TFD/Imade/Blueprints/BaseBlueprints/BP_WeaponBase.BP_WeaponBase_C|GetDamage _asbp_weapon_base) (Variables|/Game/TFD/Imade/Blueprints/BaseBlueprints/BP_WeaponBase.BP_WeaponBase_C|GetCirticalDamage _asbp_weapon_base))))
        (return)
        (elif (>= (Variables|Default|GetHp) 0.0)
          (Variables|Default|SetHp (- (Variables|Default|GetHp) (* (Variables|/Game/TFD/Imade/Blueprints/BaseBlueprints/BP_WeaponBase.BP_WeaponBase_C|GetDamage _asbp_weapon_base) (Variables|/Game/TFD/Imade/Blueprints/BaseBlueprints/BP_WeaponBase.BP_WeaponBase_C|GetCirticalDamage _asbp_weapon_base))))
          (return)))
      (else
        (Variables|/Game/TFD/Imade/Blueprints/BaseBlueprints/BP_WeaponBase.BP_WeaponBase_C|SetCirticalHit _asbp_weapon_base false)
        (if (>= (Variables|Default|GetShield) 0.0)
          (Variables|Default|SetShield (- (Variables|Default|GetShield) (Variables|/Game/TFD/Imade/Blueprints/BaseBlueprints/BP_WeaponBase.BP_WeaponBase_C|GetDamage _asbp_weapon_base)))
          (return)
          (elif (>= (Variables|Default|GetHp) 0.0)
            (Variables|Default|SetHp (- (Variables|Default|GetHp) (Variables|/Game/TFD/Imade/Blueprints/BaseBlueprints/BP_WeaponBase.BP_WeaponBase_C|GetDamage _asbp_weapon_base)))
            (return)))))))