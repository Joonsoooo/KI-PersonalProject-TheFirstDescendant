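; BP_Executioner is an AI enemy Blueprint that manages skill cooldowns through its Blackboard.
; BeginPlay writes CurrentMode to the Blackboard via SetMode.
; Every Tick runs a priority chain over cooldown flags for plasma, lightning, guillotine and minion-summon skills, clearing one after a fixed Delay.
; The BallLighting condition is hardwired true, so the Guillotine and both summon branches below it never run.
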(event EventBeginPlay
  (CallFunction|SetMode))

(event EventTick
  (params (DeltaSeconds :type Float%20%28single-precision%29))
  (CallFunction|ManageSkillsCooltime))

(event Custom|Manage%20Skills%20Cooltime
  (bind _returnvalue (AI|GetBlackboard 0))
  (bind _returnvalue_2 (Utilities|Name|MakeLiteralName "CoolTime_PlasmaPulse"))
  (bind _returnvalue_3 (AI|GetBlackboard 0))
  (bind _returnvalue_4 (Utilities|Name|MakeLiteralName "CoolTime_PlasmaBeam"))
  (bind _returnvalue_5 (Utilities|Name|MakeLiteralName "CoolTime_SummonFlyMinions"))
  (bind _returnvalue_6 (AI|GetBlackboard 0))
  (bind _returnvalue_7 (Utilities|Name|MakeLiteralName "CoolTime_Guillotine"))
  (bind _returnvalue_8 (AI|GetBlackboard 0))
  (if (ScalableFloat|GetValueasBool _returnvalue_8 _returnvalue_2)
    (Utilities|FlowControl|Delay 5.0)
    (AI|Components|Blackboard|SetValueasBool _returnvalue_8 _returnvalue_2 false)
    (elif (ScalableFloat|GetValueasBool _returnvalue_3 _returnvalue_4)
      (Utilities|FlowControl|Delay 5.0)
      (AI|Components|Blackboard|SetValueasBool _returnvalue_3 _returnvalue_4 false)
      (elif true
        (Utilities|FlowControl|Delay 5.0)
        (AI|Components|Blackboard|SetValueasBool (AI|GetBlackboard 0) (Utilities|Name|MakeLiteralName "CoolTime_BallLighting") false)
        (elif (ScalableFloat|GetValueasBool _returnvalue_6 _returnvalue_7)
          (Utilities|FlowControl|Delay 5.0)
          (AI|Components|Blackboard|SetValueasBool _returnvalue_6 _returnvalue_7 false)
          (elif true
            (Utilities|FlowControl|Delay 2e+01)
            (AI|Components|Blackboard|SetValueasBool (AI|GetBlackboard 0) (Utilities|Name|MakeLiteralName "CoolTime_SummonMinions") false)
            (elif (not true)
              (if (ScalableFloat|GetValueasBool _returnvalue _returnvalue_5)
                (Utilities|FlowControl|Delay 6e+01)
                (AI|Components|Blackboard|SetValueasBool _returnvalue _returnvalue_5 false)))))))))

(fn ConstructionScript)

(fn SetMode
  (AI|Components|Blackboard|SetValueasEnum (AI|GetBlackboard 0) (Utilities|Name|MakeLiteralName "CurrentMode") (Variables|Default|GetCurrentMode))
  (return))