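; Child weapon Blueprint that overrides Fire to shoot bullets, leaving Reload to its parent.
; Fire attaches muzzle flash and trail Niagara effects before the ammo check, so they spawn even when empty.
; With ammo, it returns a forward line trace hit and launches a Bullet actor carrying damage and critical stats along the crosshair direction.
; Each shot spends ammo and blocks firing until ShotDelay elapses, re-enabling only if ammo remains.
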(event EventBeginPlay)

(event Collision|EventActorBeginOverlap
  (params (OtherActor :type Actor%20Object%20Reference)))

(event EventTick
  (params (DeltaSeconds :type Float%20%28single-precision%29)))

(event EventShotDelay
  (Utilities|FlowControl|Delay (Variables|Default|GetShotDelay))
  (if (Variables|Default|GetHaveCurrentAmmo)
    (Variables|Default|SetCanFire true)))

(fn ConstructionScript
  (|CallParentFunction))

(fn Reload
  (|CallParentFunction))

(fn Fire
  (params (CrosshairTransform :type Transform))
  (bind (_location _rotation) (Math|Transform|BreakTransform CrosshairTransform))
  (bind _skeletalmesh (Variables|Default|GetSkeletalMesh))
  (bind _returnvalue (Math|Vector|GetForwardVector _rotation))
  (bind _output_get (Variables|Default|SetCrosshair%20Transform CrosshairTransform))
  (Niagara|SpawnSystemAttached "/Game/TFD/VFX/sA_Megapack_v1/sA_ShootingVfxPack/FX/NiagaraSystems/NS_AR_Muzzleflash_2_ONCE.NS_AR_Muzzleflash_2_ONCE" _skeletalmesh "Muzzle" (.location _output_get) "0, 0, 0" "KeepWorldPosition" true)
  (Niagara|SpawnSystemAttached "/Game/TFD/Imade/VFX/NS_BulletTrail.NS_BulletTrail" _skeletalmesh "Muzzle" (.location _output_get) "0, 0, 0" "KeepWorldPosition" true)
  (if (> (Variables|Default|GetCurrent%20Ammo) 0)
    (Utilities|FlowControl|Sequence
      (:then_0
        (bind _outhit (Collision|LineTraceByChannel _location (+ (* _returnvalue 5e+03) _location) "TraceTypeQuery1" false (Utilities|Array|MakeArray (Components|GetOwner) (Game|GetPlayerCharacter 0)) "None"))
        (bind _returnvalue_2 (Game|SpawnActorfromClass (Variables|Default|GetBullet) CrosshairTransform "Undefined" 0 0))
        (Variables|/Game/TFD/Imade/Blueprints/BaseBlueprints/BP_BulletBase.BP_BulletBase_C|SetGetDamage _returnvalue_2 (Variables|Default|GetDamage))
        (Variables|/Game/TFD/Imade/Blueprints/BaseBlueprints/BP_BulletBase.BP_BulletBase_C|SetGetCriticalHitChance%20 _returnvalue_2 (Variables|Default|GetCriticalHitChance%20))
        (Variables|/Game/TFD/Imade/Blueprints/BaseBlueprints/BP_BulletBase.BP_BulletBase_C|SetGetCirticalDamage _returnvalue_2 (Variables|Default|GetCirticalDamage))
        (Variables|/Script/Engine.MovementComponent|SetVelocity (Variables|/Game/TFD/Imade/Blueprints/BaseBlueprints/BP_BulletBase.BP_BulletBase_C|GetProjectileMovement _returnvalue_2) (* _returnvalue (Variables|Default|GetBulletSpeed))))
      (:then_1
        (bind _output_get_2 (Variables|Default|SetCurrent%20Ammo (- (Variables|Default|GetCurrent%20Ammo) 1)))
        (Variables|Default|SetHaveCurrentAmmo (> _output_get_2 0))
        (Variables|Default|SetCanFire false)
        (CallFunction|ShotDelay)
        (return _outhit)))))